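; Interactable .50 Cal gun actor that gives the player that weapon.
; On BeginPlay it runs the parent logic, then spawns a separate magazine actor and attaches it to the Mag socket on its Cube component.
; Its Interact event sets the interacting player's weapon to the 50Cal type.
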(event `self.ReceiveBeginPlay`
  (`parent.ReceiveBeginPlay`)
  (bind _returnvalue (`|SpawnActorFromClass` "/Game/Guns/50-Cal/BP_50CalMag.BP_50CalMag_C" (`KismetMathLibrary.MakeTransform` (0.0 0.0 0.0)) "Undefined" "MultiplyWithRoot" null null))
  (`self.K2_AttachToComponent` _returnvalue (`self.Cube`) "Mag" "KeepRelative" "KeepRelative" "KeepRelative" true))

(event `/Game/Blueprints/BP_InteractionSystem.Interact`
  (params (Player :type "/Game/Blueprints/BP_Player Object Reference"))
  (`/Game/Blueprints/BP_Player.SetWeapon` Player "/Game/Blueprints/Data/DataAssets/50-Cal.50-Cal"))

(fn `UserConstructionScript`
  (`parent.UserConstructionScript`))