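; BP_ClassifiedFile is an interactable classified file pickup that reveals the level exit when the player uses it.
; On Interact it destroys itself, then finds a BP_Exit actor by class and, if valid, calls its Visible function.
; It has no other active logic, as BeginPlay, overlap and Tick are disabled placeholders.
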(event `/Game/Blueprints/BP_InteractionSystem.Interact`
  (params (Player :type "/Game/Blueprints/BP_Player Object Reference"))
  (`self.K2_DestroyActor`)
  (bind _returnvalue (`GameplayStatics.GetActorOfClass` "/Game/Blueprints/BP_Exit.BP_Exit_C"))
  (`/Engine/EditorBlueprintResources/StandardMacros.IsValid` _returnvalue
    (:`Is Valid`
      (`/Game/Blueprints/BP_Exit.Visible` _returnvalue))))

(fn `UserConstructionScript`
  (`parent.UserConstructionScript`))