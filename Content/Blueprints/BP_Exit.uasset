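; Exit actor that stays hidden and non-collidable from BeginPlay until its Visible event is called.
; Visible restores query and physics collision on the Cube and Sphere and shows the Cube, without propagating to the children that were hidden with it at start.
; Interact is a placeholder that only prints "Exit".
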(event `self.ReceiveBeginPlay`
  (bind _cube (`self.Cube`))
  (`parent.ReceiveBeginPlay`)
  (`PrimitiveComponent.SetCollisionEnabled` _cube "NoCollision")
  (`PrimitiveComponent.SetCollisionEnabled` (`self.Sphere`) "NoCollision")
  (`SceneComponent.SetVisibility` _cube false true))

(event `Visible`
  (bind _cube (`self.Cube`))
  (`PrimitiveComponent.SetCollisionEnabled` _cube "QueryAndPhysics")
  (`PrimitiveComponent.SetCollisionEnabled` (`self.Sphere`) "QueryAndPhysics")
  (`SceneComponent.SetVisibility` _cube true false))

(event `/Game/Blueprints/BP_InteractionSystem.Interact`
  (params (Player :type "/Game/Blueprints/BP_Player Object Reference"))
  (`KismetSystemLibrary.PrintString` "Exit"))

(fn `UserConstructionScript`
  (`parent.UserConstructionScript`))