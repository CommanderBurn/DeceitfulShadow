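; AI controller for BP_Enemy that runs its behavior tree and manages the Roam, Alert and Hostile states.
; SetAIState mirrors the state to the pawn and blackboard and adjusts walk speed, running faster when Hostile.
; Perception updates from a non-crouching player move a roaming enemy to Alert and store the player's location as the target.
; TalkTrigger sets the blackboard's talking flag.
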(event `self.ReceiveBeginPlay`
  (bind _blackboardcomponent (`self.UseBlackboard` "/Game/Blueprints/AI/BB_EnemyBehavior.BB_EnemyBehavior"))
  (set `self.Blackboard Component` _blackboardcomponent)
  (`self.RunBehaviorTree` "/Game/Blueprints/AI/BT_EnenmyBehavior.BT_EnenmyBehavior"))

(event `SetAIState`
  (params (State :type "/Game/Blueprints/AI/BehaviorState Enum" :default "NewEnumerator0"))
  (bind _asbp_enemy (cast `/Game/Blueprints/BP_Enemy` (`self.K2_GetPawn`)))
  (`/Engine/EditorBlueprintResources/StandardMacros.IsValid` _asbp_enemy
    (:`Is Valid`
      (bind _output_get (set `/Game/Blueprints/BP_Enemy.State` State _asbp_enemy))
      (set `self.Behavior` State)
      (`BlackboardComponent.SetValueAsEnum` (`self.Blackboard Component`) "Behavior" State)
      (switch `/Game/Blueprints/AI/BehaviorState` _output_get
        (:`NewEnumerator0`
          (bind _charactermovement (`Character.CharacterMovement` _asbp_enemy))
          (set `CharacterMovementComponent.MaxWalkSpeed` 300.0 _charactermovement))
        (:`NewEnumerator1`
          (set `CharacterMovementComponent.MaxWalkSpeed` 300.0 _charactermovement))
        (:`NewEnumerator2`
          (set `CharacterMovementComponent.MaxWalkSpeed` 600.0 _charactermovement))))))

(event `TalkTrigger`
  (params (`Talk?` :type Boolean))
  (`BlackboardComponent.SetValueAsBool` (`self.Blackboard Component`) "Talking?" `Talk?`))

(event `self.AIPerception.OnTargetPerceptionUpdated`
  (params (Actor :type "Actor Object Reference") (Stimulus :type "AIStimulus Structure"))
  (bind _returnvalue (`GameplayStatics.GetPlayerCharacter` 0))
  (bind _asbp_player (cast `/Game/Blueprints/BP_Player` _returnvalue))
  (`/Engine/EditorBlueprintResources/StandardMacros.IsValid` _asbp_player
    (:`Is Valid`
      (if (and (== Actor _returnvalue) (not (`/Game/Blueprints/BP_Player.CrouchToggle` _asbp_player)))
        (if (`|EnumEquality` (`self.Behavior`) "NewEnumerator0")
          (bind _asbp_player_2 (cast `/Game/Blueprints/BP_Player` Actor))
          (`/Engine/EditorBlueprintResources/StandardMacros.IsValid` _asbp_player_2
            (:`Is Valid`
              (`BlackboardComponent.SetValueAsVector` (`self.Blackboard Component`) "TargetLocation" (`SceneComponent.K2_GetComponentLocation` (`Character.Mesh` _asbp_player_2)))
              (`self.SetAIState` "NewEnumerator1"))))))))

(fn `UserConstructionScript`)