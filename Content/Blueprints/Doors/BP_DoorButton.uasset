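; BP_DoorButton is an interactable button that toggles a set of linked doors.
; On Interact it loops over its Doors array, inverts each door's CloseToggle flag and calls OpenClose on it.
; Each door flips from its own current state, so doors in mixed states stay opposite to one another.
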(event `/Game/Blueprints/BP_InteractionSystem.Interact`
  (params (Player :type "/Game/Blueprints/BP_Player Object Reference"))
  (for _array_element (`self.Doors`)
    (set `/Game/Blueprints/Doors/BP_Doors.CloseToggle` (not (`/Game/Blueprints/Doors/BP_Doors.CloseToggle` _array_element)) _array_element)
    (`/Game/Blueprints/Doors/BP_Doors.Open/Close` _array_element)))

(fn `UserConstructionScript`
  (`parent.UserConstructionScript`))