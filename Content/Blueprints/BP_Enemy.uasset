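; Enemy character that roams, turns hostile and holds scripted conversations with other enemies, driven through BP_AIControl.
; Tick uses player distance per state: Roam sets CanKill, Alert escalates to Hostile when close, and Hostile faces the player.
; Talk pairs with a nearby enemy, and Speak steps through timed Script lines, alternating speakers and showing text on BP_Player within range.
; A reversible timeline handles turning in place; Fire calls FireGun.
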(event `self.ReceiveBeginPlay`
  ;[0.135 0.03379 0.15 0.5] Initialization
  (`parent.ReceiveBeginPlay`)
  (bind _asbp_aicontrol (cast `/Game/Blueprints/AI/BP_AIControl` (`AIBlueprintHelperLibrary.GetAIController` self)))
  (`/Engine/EditorBlueprintResources/StandardMacros.IsValid` _asbp_aicontrol
    (:`Is Valid`
      (`/Game/Blueprints/AI/BP_AIControl.SetAIState` _asbp_aicontrol (`self.State`))
      (set `self.BP AIControl` _asbp_aicontrol))))

(event `Action`)

(event `Fire`
  ;[0.07004 0.15 0 0.5] Gun Logic
  (`self.FireGun`))

(event `self.ReceiveTick`
  (params (DeltaSeconds :type "Float (single-precision)"))
  (bind _returnvalue (`self.GetDistanceTo` (`GameplayStatics.GetPlayerCharacter` 0)))
  ;[0.15 0.1297 0 0.5] AI Behavior Updates
  (`parent.ReceiveTick` DeltaSeconds)
  (switch `/Game/Blueprints/AI/BehaviorState` (`self.State`)
    (:`NewEnumerator0`
      (set `self.CanKill?` (<= _returnvalue 100.0)))
    (:`NewEnumerator1`
      (if (<= _returnvalue 200.0)
        (`/Game/Blueprints/AI/BP_AIControl.SetAIState` (`self.BP AIControl`) "NewEnumerator2")
        (`MovementComponent.StopMovementImmediately` (`self.CharacterMovement`))))
    (:`NewEnumerator2`
      (`self.K2_SetActorRotation` (`KismetMathLibrary.FindLookAtRotation` (`self.K2_GetActorLocation`) (`self.K2_GetActorLocation` (`GameplayStatics.GetPlayerCharacter` 0)))))))

(event `TurnAround`
  ;[1 1 1] StillMovement
  (if (`self.IsTurned?`)
    (bind (_direction _newtrack_0) (`Timeline|Turn` :!via `ReverseFromEnd` :!label _label)
      (:`Update`
        (if (not (`self.Talking?`))
          (`SceneComponent.K2_SetRelativeRotation` (`self.CapsuleComponent`) (`KismetMathLibrary.MakeRotator` 0.0 0.0 _newtrack_0) false false)))
      (:`Finished`
        (set `self.IsTurned?` (not (`self.IsTurned?`)))))
    (else
      (goto _label :!via `PlayFromStart`))))

(event `RecieveTalk`
  (params (TalkingEnemy :type "/Game/Blueprints/BP_Enemy Object Reference"))
  ;[0 0.008211 0.15 0.5] Talking Logic
  (set `self.As BP Enemy` TalkingEnemy)
  (`self.K2_SetActorRotation` (`KismetMathLibrary.FindLookAtRotation` (`self.K2_GetActorLocation`) (`self.K2_GetActorLocation` TalkingEnemy)))
  (bind _output_get (set `self.Talking?` true))
  (`/Game/Blueprints/AI/BP_AIControl.TalkTrigger` (`self.BP AIControl`) _output_get))

(event `Speak`
  (bind _as_bp_enemy (`self.As BP Enemy`))
  (bind _script (`self.Script`))
  (bind (_key _value) (`BlueprintMapLibrary.Map_GetKeyValueByIndex` _script (`self.ScriptIndex`)))
  ;[0 0.008211 0.15 0.5] Talking Logic
  (`/Engine/EditorBlueprintResources/StandardMacros.IsValid` _as_bp_enemy
    (:`Is Valid`
      (if (== (`BlueprintMapLibrary.Map_Length` _script) (`self.ScriptIndex`))
        (if (not (`/Game/Blueprints/BP_Enemy.CurrentTalking?` _as_bp_enemy))
          (`self.TalkSwitch` false)
          (`self.TalkSwitch` _as_bp_enemy false)
          (set `self.ScriptIndex` 0)
          (set `/Game/Blueprints/BP_Enemy.ScriptIndex` 0 _as_bp_enemy)
          (set `self.CurrentTalking?` false)
          (`self.HandleTextView` ""))
        (else
          (`self.HandleTextView` (`KismetTextLibrary.Conv_StringToText` _key) (<= (`self.GetDistanceTo` (`GameplayStatics.GetPlayerCharacter` 0)) 1000.0))
          (`KismetSystemLibrary.Delay` _value)
          (set `/Game/Blueprints/BP_Enemy.CurrentTalking?` true _as_bp_enemy)
          (set `self.CurrentTalking?` false)
          (`/Engine/EditorBlueprintResources/StandardMacros.IncrementInt` (`self.ScriptIndex`)))))))

(event `Talk`
  ;[0 0.008211 0.15 0.5] Talking Logic
  (bind _outactors (`KismetSystemLibrary.SphereOverlapActors` (`self.K2_GetActorLocation`) 200.0 (`|MakeArray` "ObjectTypeQuery3" :!type "EObjectTypeQuery Enum") "BP_Enemy_C" (`|MakeArray` self :!type "Actor Object Reference")))
  (for _array_element _outactors
    (bind _asbp_enemy (cast `/Game/Blueprints/BP_Enemy` _array_element))
    (`/Engine/EditorBlueprintResources/StandardMacros.IsValid` _asbp_enemy
      (:`Is Valid`
        (bind _output_get (set `self.As BP Enemy` _asbp_enemy))
        (`self.RecieveTalk` _output_get self)
        (`self.K2_SetActorRotation` (`KismetMathLibrary.FindLookAtRotation` (`self.K2_GetActorLocation`) (`self.K2_GetActorLocation` _asbp_enemy)))
        (break))))
  (bind _output_get_2 (set `self.Talking?` true))
  (`/Game/Blueprints/AI/BP_AIControl.TalkTrigger` (`self.BP AIControl`) _output_get_2))

(fn `HandleTextView`
  (params (InText :type Text) (ShowText :type Boolean))
  (bind _asbp_player (cast `/Game/Blueprints/BP_Player` (`GameplayStatics.GetPlayerCharacter` 0)))
  (`/Engine/EditorBlueprintResources/StandardMacros.IsValid` _asbp_player
    (:`Is Valid`
      (if ShowText
        (bind _conversationtext (`/Game/Blueprints/BP_Player.ConversationText` _asbp_player))
        (`/Game/Blueprints/WB_ConservationText.Visible` _conversationtext "Visible")
        (`/Game/Blueprints/WB_ConservationText.SetText` _conversationtext InText)
        (else
          (`/Game/Blueprints/WB_ConservationText.Visible` _conversationtext "Hidden")
          (`/Game/Blueprints/WB_ConservationText.SetText` _conversationtext ""))))))

(fn `TalkSwitch`
  (params (`Talk?` :type Boolean))
  (set `self.Talking?` `Talk?`)
  (`/Game/Blueprints/AI/BP_AIControl.TalkTrigger` (`self.BP AIControl`) `Talk?`))

(fn `UserConstructionScript`
  (`parent.UserConstructionScript`))