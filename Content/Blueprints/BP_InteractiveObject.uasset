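; BP_InteractiveObject is an interactive actor that shows a widget and registers itself with the player when they are in range.
; While not held, its sphere overlap toggles the widget for the player character and sets or clears InteractiveActor on BP_Player.
; DestroyObject destroys its directly attached actors, then the object itself.
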(event `self.Sphere.OnComponentBeginOverlap`
  (params (OverlappedComponent :type "PrimitiveComponent Object Reference") (OtherActor :type "Actor Object Reference") (OtherComp :type "PrimitiveComponent Object Reference") (OtherBodyIndex :type Integer) (bFromSweep :type Boolean) (SweepResult :type "HitResult Structure (by ref)"))
  (if (not (`self.IsHeld?`))
    (`/Engine/EditorBlueprintResources/StandardMacros.IsValid` OtherActor
      (:`Is Valid`
        (if (== OtherActor (`GameplayStatics.GetPlayerCharacter` 0))
          (`SceneComponent.SetVisibility` (`self.Widget`) true false)
          (bind _asbp_player (cast `/Game/Blueprints/BP_Player` OtherActor))
          (`/Engine/EditorBlueprintResources/StandardMacros.IsValid` _asbp_player
            (:`Is Valid`
              (set `/Game/Blueprints/BP_Player.InteractiveActor` self _asbp_player))))))))

(event `self.Sphere.OnComponentEndOverlap`
  (params (OverlappedComponent :type "PrimitiveComponent Object Reference") (OtherActor :type "Actor Object Reference") (OtherComp :type "PrimitiveComponent Object Reference") (OtherBodyIndex :type Integer))
  (if (not (`self.IsHeld?`))
    (`/Engine/EditorBlueprintResources/StandardMacros.IsValid` OtherActor
      (:`Is Valid`
        (if (== OtherActor (`GameplayStatics.GetPlayerCharacter` 0))
          (`SceneComponent.SetVisibility` (`self.Widget`) false false)
          (bind _asbp_player (cast `/Game/Blueprints/BP_Player` OtherActor))
          (`/Engine/EditorBlueprintResources/StandardMacros.IsValid` _asbp_player
            (:`Is Valid`
              (set `/Game/Blueprints/BP_Player.InteractiveActor` null _asbp_player))))))))

(event `DestroyObject`
  (for _array_element (`self.GetAttachedActors` true)
    (`self.K2_DestroyActor` _array_element))
  (`self.K2_DestroyActor`))

(fn `UserConstructionScript`)