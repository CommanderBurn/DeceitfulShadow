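; Player character with movement, interaction, weapons, aiming and a minimap.
; A top-down scene capture feeds the minimap render target, hiding ceiling actors and following camera yaw.
; SetWeapon attaches the gun model and swaps animation class; shooting spawns bullets along control rotation, or unarmed, ragdolls enemies flagged CanKill.
; Aiming shows a reticle and shifts the camera, while crouch only toggles transparent and dark-aura materials.
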(event `self.ReceiveBeginPlay`
  ;[0.15 0 0.1425 0.5] Initialization
  (bind _returnvalue (`|CreateWidget` "/Game/Blueprints/WB_ConservationText.WB_ConservationText_C"))
  (bind _output_get (set `self.ConversationText` _returnvalue))
  (`UserWidget.AddToViewport` _output_get 0)
  (`EnhancedInputSubsystemInterface.AddMappingContext` (pcsubsystem `EnhancedInputLocalPlayerSubsystem` (`GameplayStatics.GetPlayerController` 0)) "/Game/Input/IMC_Controls.IMC_Controls" 0 (struct))
  (set `CharacterMovementComponent.bOrientRotationToMovement` true (`self.CharacterMovement`))
  (`self.SetWeapon` (`self.Weapon`))
  (if (`self.IsPlayerControlled`)
    (set `SceneCaptureComponent2D.TextureTarget` "/Game/Texture/RT_Minimap.RT_Minimap" (`self.SceneCaptureComponent2D`)))
  (bind _outactors (`GameplayStatics.GetAllActorsOfClass` "/Game/Blueprints/BP_Ceiling.BP_Ceiling_C"))
  (for _array_element _outactors
    (`SceneCaptureComponent.HideActorComponents` (`self.SceneCaptureComponent2D`) _array_element false))
  (bind _outactors_2 (`GameplayStatics.GetAllActorsOfClass` "/Game/Blueprints/Lights/BP_CeilingLight.BP_CeilingLight_C"))
  (for _array_element_2 _outactors_2
    (`SceneCaptureComponent.HideActorComponents` (`self.SceneCaptureComponent2D`) _array_element_2 false))
  (bind _returnvalue_2 (`|CreateWidget` "/Game/Blueprints/WB_Minimap.WB_Minimap_C"))
  (set `self.MapWidget` _returnvalue_2)
  (`UserWidget.AddToViewport` _returnvalue_2 0)
  (`MeshComponent.SetOverlayMaterial` (`self.Mesh`) null))

(event `EnhancedInput|/Game/Input/Actions/IA_Move`
  (params (ActionValue :type "Vector2D Structure") (ElapsedSeconds :type "Float (double-precision)") (TriggeredSeconds :type "Float (double-precision)") (InputAction :type "InputAction Object Reference" :default "/Game/Input/Actions/IA_Move.IA_Move"))
  (bind _returnvalue (`self.GetController`))
  ;[0 0.01814 0.15 0.5] Controls
  (:`Triggered`
    (`self.AddMovementInput` (`self.GetActorForwardVector` _returnvalue) ActionValue_Y)
    (`self.AddMovementInput` (`self.GetActorRightVector` _returnvalue) ActionValue_X)))

(event `EnhancedInput|/Game/Input/Actions/IA_Action`
  (params (ActionValue :type Boolean) (ElapsedSeconds :type "Float (double-precision)") (TriggeredSeconds :type "Float (double-precision)") (InputAction :type "InputAction Object Reference" :default "/Game/Input/Actions/IA_Action.IA_Action"))
  (bind _interactiveactor (`self.InteractiveActor`))
  ;[0 0.01814 0.15 0.5] Controls
  (:`Started`
    (`/Engine/EditorBlueprintResources/StandardMacros.IsValid` _interactiveactor
      (:`Is Valid`
        (if (`KismetSystemLibrary.DoesImplementInterface` _interactiveactor "/Game/Blueprints/BP_InteractionSystem.BP_InteractionSystem_C")
          (message `/Game/Blueprints/BP_InteractionSystem.Interact` _interactiveactor self))))))

(event `self.ReceiveTick`
  (params (DeltaSeconds :type "Float (single-precision)"))
  (bind (_returnvalue_roll _returnvalue_pitch _returnvalue_yaw) (`KismetMathLibrary.BreakRotator` (`self.GetControlRotation`)))
  (`SceneComponent.K2_SetWorldRotation` (`self.SceneCaptureComponent2D`) (`KismetMathLibrary.MakeRotator` 0.0 -90.0 _returnvalue_yaw) false false))

(event `EnhancedInput|/Game/Input/Actions/IA_Look`
  (params (ActionValue :type "Vector2D Structure") (ElapsedSeconds :type "Float (double-precision)") (TriggeredSeconds :type "Float (double-precision)") (InputAction :type "InputAction Object Reference" :default "/Game/Input/Actions/IA_Look.IA_Look"))
  ;[0 0.01814 0.15 0.5] Controls
  (:`Triggered`
    (`self.AddControllerYawInput` ActionValue_X)
    (`self.AddControllerPitchInput` ActionValue_Y)))

(event `EnhancedInput|/Game/Input/Actions/IA_Map`
  (params (ActionValue :type Boolean) (ElapsedSeconds :type "Float (double-precision)") (TriggeredSeconds :type "Float (double-precision)") (InputAction :type "InputAction Object Reference" :default "/Game/Input/Actions/IA_Map.IA_Map"))
  ;[0 0.01814 0.15 0.5] Controls
  (:`Started`
    (`/Game/Blueprints/WB_Minimap.ToggleFullMap` (`self.MapWidget`))))

(event `EnhancedInput|/Game/Input/Actions/IA_Crouch`
  (params (ActionValue :type Boolean) (ElapsedSeconds :type "Float (double-precision)") (TriggeredSeconds :type "Float (double-precision)") (InputAction :type "InputAction Object Reference" :default "/Game/Input/Actions/IA_Crouch.IA_Crouch"))
  (bind _mesh (`self.Mesh`))
  (bind _mesh_2 (`self.Mesh`))
  ;[0 0.01814 0.15 0.5] Controls
  (:`Started`
    (bind _output_get (set `self.CrouchToggle` (not (`self.CrouchToggle`))))
    (if _output_get
      (`MeshComponent.SetOverlayMaterial` _mesh "/Game/Texture/DarkAuraMaterial.DarkAuraMaterial")
      (`PrimitiveComponent.SetMaterial` _mesh 0 "/Game/Texture/Transparency1.Transparency1")
      (`PrimitiveComponent.SetMaterial` _mesh 1 "/Game/Texture/Transparency2.Transparency2")
      (else
        (`MeshComponent.SetOverlayMaterial` _mesh_2 null)
        (`PrimitiveComponent.SetMaterial` _mesh_2 0 "/Game/Characters/Mannequins/Materials/Manny/MI_Manny_01_New.MI_Manny_01_New")
        (`PrimitiveComponent.SetMaterial` _mesh_2 1 "/Game/Characters/Mannequins/Materials/Manny/MI_Manny_02_New.MI_Manny_02_New")))))

(event `EnhancedInput|/Game/Input/Actions/IA_Shoot`
  (params (ActionValue :type Boolean) (ElapsedSeconds :type "Float (double-precision)") (TriggeredSeconds :type "Float (double-precision)") (InputAction :type "InputAction Object Reference" :default "/Game/Input/Actions/IA_Shoot.IA_Shoot"))
  ;[0 0.01814 0.15 0.5] Controls
  (:`Triggered`
    (`/Engine/EditorBlueprintResources/StandardMacros.IsValid` (`self.Weapon`)
      (:`Is Valid`
        (`self.FireGun`)
        (set `self.bUseControllerRotationYaw` true))
      (:`Is Not Valid`
        (bind _outactors (`GameplayStatics.GetAllActorsOfClass` "/Game/Blueprints/BP_Enemy.BP_Enemy_C"))
        (for _array_element _outactors
          (if (`/Game/Blueprints/BP_Enemy.CanKill?` _array_element)
            (`PrimitiveComponent.SetSimulatePhysics` (`Character.Mesh` _array_element) true)
            (`PrimitiveComponent.SetCollisionEnabled` (`Character.CapsuleComponent` _array_element) "NoCollision"))))))
  (:`Completed`
    (set `self.bUseControllerRotationYaw` false)))

(event `EnhancedInput|/Game/Input/Actions/IA_Aim`
  (params (ActionValue :type Boolean) (ElapsedSeconds :type "Float (double-precision)") (TriggeredSeconds :type "Float (double-precision)") (InputAction :type "InputAction Object Reference" :default "/Game/Input/Actions/IA_Aim.IA_Aim"))
  ;[0 0.01814 0.15 0.5] Controls
  (:`Triggered`
    (bind _returnvalue (`|CreateWidget` "/Game/Blueprints/WB_Reticle.WB_Reticle_C"))
    (set `self.Reticle` _returnvalue)
    (`UserWidget.AddToViewport` _returnvalue 0)
    (set `self.bUseControllerRotationYaw` true)
    (`self.Camera Closer` true))
  (:`Completed`
    (set `self.bUseControllerRotationYaw` false)
    (bind _foundwidgets (`WidgetBlueprintLibrary.GetAllWidgetsOfClass` "/Game/Blueprints/WB_Reticle.WB_Reticle_C"))
    (for _array_element _foundwidgets
      (`Widget.RemoveFromParent` _array_element)
      (`self.Camera Closer` false))))

(event `Camera Closer`
  (params (`Closer?` :type Boolean))
  (bind _camera (`self.Camera`))
  ;[0.15 0.008281 0.008281 0.5] Gun Logic
  (`SceneComponent.K2_SetRelativeLocation` _camera (`KismetMathLibrary.VInterpTo` (`SceneComponent.RelativeLocation` _camera) (`KismetMathLibrary.SelectVector` (50.0 50.0 50.0) (0.0 0.0 0.0) `Closer?`)) false false))

(event `FireGun`
  (bind _returnvalue_location (`KismetMathLibrary.BreakTransform` (`SceneComponent.GetSocketTransform` (`self.Gun`) "Muzzle" "RTS_World")))
  ;[0.15 0.008281 0.008281 0.5] Gun Logic
  (`|PlayMontage` (`self.Mesh`) "/Game/Characters/Mannequins/Anims/Pistol/MM_Pistol_Fire_Montage.MM_Pistol_Fire_Montage"
    (:`then`
      (`|SpawnActorFromClass` "/Game/Blueprints/BP_Bullet.BP_Bullet_C" (`KismetMathLibrary.MakeTransform` _returnvalue_location (`self.GetControlRotation`)) "Undefined" "MultiplyWithRoot" null self))))

(fn `GetBulletLocation`
  (returns (BulletLoc :type "Vector Structure"))
  (locals (Loc :type "Vector Structure" :default (0.0 0.0 0.0)))
  (bind _returnvalue (`GameplayStatics.GetPlayerController` 0))
  (bind (_sizex _sizey) (`PlayerController.GetViewportSize` _returnvalue))
  (bind (_worldlocation _worlddirection) (`PlayerController.DeprojectScreenPositionToWorld` _returnvalue (`KismetMathLibrary.Conv_IntToDouble` (/ _sizex 2)) (`KismetMathLibrary.Conv_IntToDouble` (/ _sizey 2))))
  (bind (_outhit _returnvalue_2) (`KismetSystemLibrary.LineTraceSingleForObjects` :`Start` (+ _worldlocation (* _worlddirection 400.0)) :`End` (+ _worldlocation (* _worlddirection 3000.0)) :`ObjectTypes` (`|MakeArray` "ObjectTypeQuery4" :!type "EObjectTypeQuery Enum") :`DrawDebugType` "ForDuration"))
  (if _returnvalue_2
    (bind (_bblockinghit _binitialoverlap _time _distance _location _impactpoint _normal _impactnormal _physmat _hitactor _hitcomponent _hitbonename _bonename _hititem _elementindex _faceindex _tracestart _traceend) (`GameplayStatics.BreakHitResult` _outhit))
    (set `local.Loc` _impactpoint)
    (else
      (set `local.Loc` _traceend)))
  (return (`local.Loc`)))

(fn `SetWeapon`
  (params (Weapon :type "/Game/Blueprints/Data/GunData Object Reference"))
  (bind _gunactor (`self.GunActor`))
  (`/Engine/EditorBlueprintResources/StandardMacros.IsValid` _gunactor
    (:`Is Valid`
      (`/Game/Blueprints/BP_InteractiveObject.DestroyObject` _gunactor))
    (:`Is Not Valid`
      _))
  (`/Engine/EditorBlueprintResources/StandardMacros.IsValid` Weapon
    (:`Is Valid`
      (`SkeletalMeshComponent.SetAnimInstanceClass` (`self.Mesh`) (`/Game/Blueprints/Data/GunData.AnimationBP` Weapon))
      (bind _returnvalue (`|SpawnActorFromClass` (`/Game/Blueprints/Data/GunData.Model` Weapon) (`KismetMathLibrary.MakeTransform` (0.0 0.0 0.0)) "Undefined" "MultiplyWithRoot" null true null))
      (set `self.GunActor` _returnvalue)
      (`self.K2_AttachToComponent` _returnvalue (`self.Mesh`) "HandGrip_R" "KeepRelative" "KeepRelative" "KeepRelative" true)
      (set `self.Weapon` Weapon))
    (:`Is Not Valid`
      (`SkeletalMeshComponent.SetAnimInstanceClass` (`self.Mesh`) "/Game/Variant_Combat/Anims/ABP_Manny_Combat.ABP_Manny_Combat_C")
      (set `self.Weapon` null))))

(fn `UserConstructionScript`)